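; BP_Car is a car prop that randomizes its look through the GenerateRandom event, not on construction or BeginPlay.
; RandomGenerator picks a mesh variation by car type, with FullyRandom also rolling type and foliage and forcing random color.
; A dynamic material, clean or default, gets palette color plus random leaf amount, or manual paint; ambulances skip tinting.
; Optional foliage reuses the body's mesh index to match the variation, otherwise its component is destroyed.
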(event Custom|GenerateRandom
  (CallFunction|RandomGenerator))

(event EventBeginPlay)

(event Collision|EventActorBeginOverlap
  (params (OtherActor :type Actor%20Object%20Reference)))

(event EventTick
  (params (DeltaSeconds :type Float%20%28single-precision%29)))

(fn ConstructionScript)

(fn RandomGenerator
  (bind _carcolors (Variables|Colors|GetCarColors))
  (bind _car (Variables|Default|GetCar))
  (bind _foliage (Variables|Default|GetFoliage))
  (if (Variables|Control|GetFullyRandom)
    ;[1 1 1] If fully Random
    (Variables|Control|SetCarType (Utilities|Select :Index (Math|Random|RandomInteger 4) :Option%200 "NewEnumerator0" :Option%201 "NewEnumerator1" :Option%202 "NewEnumerator2" :Option%203 "NewEnumerator3"))
    (Variables|Colors|SetRandomColor true)
    (Variables|Control|SetAllowFoliage (Math|Random|RandomBool)))
  ;[1 1 1] Set Vehicle Type
  (Variables|Default|SetActiveArray (Utilities|Select :Index (Variables|Control|GetCarType) :NewEnumerator0 (Variables|Default|GetCarVariationsHatchback) :NewEnumerator1 (Variables|Default|GetCarVariationsPickup) :NewEnumerator2 (Variables|Default|GetCarVariationsWagon) :NewEnumerator3 (Variables|Default|GetCarVariationsAmbulance)))
  ;[1 1 1] Set Mesh Variation
  (bind _output_get (Variables|Default|SetMeshIndex (Math|Random|RandomInteger (Utilities|Array|Length (Variables|Default|GetActiveArray)))))
  (Components|StaticMesh|SetStaticMesh (Variables|Default|GetCar) (Utilities|Array|Get(acopy) (Variables|Default|GetActiveArray) _output_get))
  ;[1 1 1] Create Material Instance
  (bind _returnvalue (Rendering|Material|CreateDynamicMaterialInstance _car 0 (select (Variables|Control|GetCleanVersion) (Utilities|Select :Index (Variables|Control|GetCarType) :NewEnumerator0 "/Game/PostDistrict/Materials/Vehicles/MI_Hatchback_Clean.MI_Hatchback_Clean" :NewEnumerator1 "/Game/PostDistrict/Materials/Vehicles/MI_Pickup_Clean.MI_Pickup_Clean" :NewEnumerator2 "/Game/PostDistrict/Materials/Vehicles/MI_Wagon_Clean.MI_Wagon_Clean" :NewEnumerator3 "/Game/PostDistrict/Materials/Vehicles/MI_Ambulance_Clean.MI_Ambulance_Clean") (Utilities|Select :Index (Variables|Control|GetCarType) :NewEnumerator0 "/Game/PostDistrict/Materials/Vehicles/MI_Hatchback.MI_Hatchback" :NewEnumerator1 "/Game/PostDistrict/Materials/Vehicles/MI_Pickup.MI_Pickup" :NewEnumerator2 "/Game/PostDistrict/Materials/Vehicles/MI_Wagon.MI_Wagon" :NewEnumerator3 "/Game/PostDistrict/Materials/Vehicles/MI_Ambulance.MI_Ambulance")) "None" :!class /Script/Engine.PrimitiveComponent))
  (bind _output_get_2 (Variables|Default|SetCarBodyMatInst _returnvalue))
  (Rendering|Material|SetMaterial _car 0 _output_get_2)
  (if (Utilities|Enum|Equal(Enum) (Variables|Control|GetCarType) "NewEnumerator3")
    _
    (elif (Variables|Colors|GetRandomColor)
      ;[1 1 1] Generate Random Color
      (Rendering|Material|SetVectorParameterValue (Variables|Default|GetCarBodyMatInst) "AlbedoColor" (Utilities|Array|Get(acopy) _carcolors (Math|Random|RandomInteger (Utilities|Array|Length _carcolors))) :!class /Script/Engine.MaterialInstanceDynamic)
      (Rendering|Material|SetScalarParameterValue (Variables|Default|GetCarBodyMatInst) "LeafsMultiplier" (Math|Random|RandomFloatinRange 2.0 6.0) :!class /Script/Engine.MaterialInstanceDynamic)
      (else
        ;[1 1 1] Generate Color
        (Rendering|Material|SetVectorParameterValue (Variables|Default|GetCarBodyMatInst) "AlbedoColor" (Variables|Colors|GetManualCarPaintColor) :!class /Script/Engine.MaterialInstanceDynamic))))
  ;[1 1 1] Add Foliage
  (if (Variables|Control|GetAllowFoliage)
    (Components|StaticMesh|SetStaticMesh _foliage (Utilities|Array|Get(acopy) (Utilities|Select :Index (Variables|Control|GetCarType) :NewEnumerator0 (Variables|Default|GetHatchbackFol) :NewEnumerator1 (Variables|Default|GetPickupFol) :NewEnumerator2 (Variables|Default|GetWagonFol) :NewEnumerator3 (Variables|Default|GetAmbulanceFol)) (Variables|Default|GetMeshIndex)))
    (Rendering|SetVisibility _foliage true false)
    (else
      (Components|DestroyComponent (Variables|Default|GetFoliage)))))